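; Base enemy Blueprint that supplies the visual spawn, death-style dissolve and facing behavior for an enemy character.
; On BeginPlay a timeline scales the mesh through its Extend track as a spawn effect.
; A dissolve event drives the Dissolve scalar on the body and weapon dynamic materials from a timeline.
; SetFacingTarget feeds a location into Motion Warping as the FacingToTarget warp target.
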(event EventBeginPlay
  (bind _extend (Timeline|SpawnEffect PlayFromStart)
    (:Update
      (Transformation|SetRelativeScale3D (Variables|Character|GetMesh) (Math|Vector|MakeVector _extend _extend _extend)))))

(event EventStartDissolveMeshandWeaponTimeLine
  (params (DissolveMeshMaterial :type Material%20Instance%20Dynamic%20Object%20Reference) (DissolveWeaponMeshMaterial :type Material%20Instance%20Dynamic%20Object%20Reference))
  (bind _dissolvetime (Timeline|Dissolve Play)
    (:Update
      (Utilities|IsValid DissolveMeshMaterial
        (:Is%20Valid
          (Rendering|Material|SetScalarParameterValue DissolveMeshMaterial "Dissolve" _dissolvetime :!class /Script/Engine.MaterialInstanceDynamic))
        (:Is%20Not%20Valid
          _))
      (Utilities|IsValid DissolveWeaponMeshMaterial
        (:Is%20Valid
          (Rendering|Material|SetScalarParameterValue DissolveWeaponMeshMaterial "Dissolve" _dissolvetime :!class /Script/Engine.MaterialInstanceDynamic))))))

(event EventSetFacingTarget
  (params (TargetLocation :type Vector%20%28by%20ref%29 :default "0, 0, 0"))
  (Class|MotionWarpingComponent|AddorUpdateWarpTargetfromLocation (Variables|Default|GetMotionWarping) "FacingToTarget" TargetLocation))

(fn ConstructionScript)