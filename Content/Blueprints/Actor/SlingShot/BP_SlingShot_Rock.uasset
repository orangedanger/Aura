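; BP_SlingShot_Rock is a slingshot rock actor whose mesh tumbles continuously.
; BeginPlay picks a random rotation step for each of roll, pitch and yaw.
; Tick adds those steps to the mesh's world rotation every frame, without scaling by delta time, so spin speed depends on frame rate.
; The Blueprint graphs hold no movement or hit logic.
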(event EventBeginPlay
  (bind _returnvalue (Math|Random|RandomFloatinRange -5e+02 5e+02))
  (Variables|Default|SetRotation%20Roll _returnvalue)
  (Variables|Default|SetRotation%20Pitch _returnvalue)
  (Variables|Default|SetRotation%20Yaw _returnvalue))

(event Collision|EventActorBeginOverlap
  (params (OtherActor :type Actor%20Object%20Reference)))

(event EventTick
  (params (DeltaSeconds :type Float%20%28single-precision%29))
  (bind _sm_slingshotrock (Variables|Default|GetSM_SlingshotRock))
  (bind _returnvalue (Transformation|GetWorldRotation _sm_slingshotrock))
  (Transformation|SetWorldRotation (Variables|Default|GetSM_SlingshotRock) (Math|Rotator|MakeRotator (+ (.roll _returnvalue) (Variables|Default|GetRotation%20Roll)) (+ (.pitch _returnvalue) (Variables|Default|GetRotation%20Pitch)) (+ (.yaw _returnvalue) (Variables|Default|GetRotation%20Yaw))) false false))

(fn ConstructionScript)