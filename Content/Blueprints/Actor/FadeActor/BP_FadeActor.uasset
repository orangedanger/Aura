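; Actor that fades its static mesh in and out through a timeline-driven Opacity material parameter.
; Construction caches the original materials and creates dynamic instances from FadeMaterials.
; Fadein applies those instances and plays the timeline, while FadeOut reverses it.
; With VisiblityChannal enabled, either end sets Visibility collision to Ignore, and only the zero-opacity end restores the original materials.
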(event EventBeginPlay)

(event EventFadein
  (CallFunction|SetDynamicMaterial)
  (bind _opacity (Timeline|Fade Play)
    (:Update
      (for _array_element (Variables|Default|GetDynamicMaterial)
        (Rendering|Material|SetScalarParameterValue _array_element "Opacity" _opacity :!class /Script/Engine.MaterialInstanceDynamic)))
    (:Finished
      (if (Variables|Default|GetbVisiblityChannal)
        ;[1 1 1] Fade Out Finish
        (if (<= _opacity 0.0)
          (Collision|SetCollisionResponsetoChannel (Variables|Default|GetStaticMesh) "ECC_Visibility" "ECR_Ignore")
          (CallFunction|ResetMaterial)
          (else
            ;[1 1 1] Fade In Finish
            (if (>= _opacity 1.0)
              (Collision|SetCollisionResponsetoChannel (Variables|Default|GetStaticMesh) "ECC_Visibility" "ECR_Ignore"))))))))

(event EventFadeOut
  (bind _opacity (Timeline|Fade Reverse)
    (:Update
      (for _array_element (Variables|Default|GetDynamicMaterial)
        (Rendering|Material|SetScalarParameterValue _array_element "Opacity" _opacity :!class /Script/Engine.MaterialInstanceDynamic)))
    (:Finished
      (if (Variables|Default|GetbVisiblityChannal)
        ;[1 1 1] Fade Out Finish
        (if (<= _opacity 0.0)
          (Collision|SetCollisionResponsetoChannel (Variables|Default|GetStaticMesh) "ECC_Visibility" "ECR_Ignore")
          (CallFunction|ResetMaterial)
          (else
            ;[1 1 1] Fade In Finish
            (if (>= _opacity 1.0)
              (Collision|SetCollisionResponsetoChannel (Variables|Default|GetStaticMesh) "ECC_Visibility" "ECR_Ignore"))))))))

(fn ConstructionScript
  (Utilities|Array|Clear (Variables|Default|GetDynamicMaterial))
  (Variables|Default|SetOrginalMaterials (Rendering|Material|GetMaterials (Variables|Default|GetStaticMesh)))
  (for (_array_element _array_index) (Variables|Default|GetFadeMaterials)
    (bind _returnvalue (Rendering|Material|CreateDynamicMaterialInstance (Variables|Default|GetStaticMesh) _array_index _array_element "None" :!class /Script/Engine.PrimitiveComponent))
    (Utilities|Array|Add (Variables|Default|GetDynamicMaterial) _returnvalue)))

(fn SetDynamicMaterial
  (for (_array_element _array_index) (Variables|Default|GetDynamicMaterial)
    (Rendering|Material|SetMaterial (Variables|Default|GetStaticMesh) _array_index _array_element)))

(fn ResetMaterial
  (for (_array_element _array_index) (Variables|Default|GetOrginalMaterials)
    (Rendering|Material|SetMaterial (Variables|Default|GetStaticMesh) _array_index _array_element)))