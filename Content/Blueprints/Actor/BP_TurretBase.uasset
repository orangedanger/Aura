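; Base turret actor that tracks tagged enemies inside an attack-radius sphere and selects one as its target.
; Sphere overlaps maintain the enemy list, and a looping timer starts at BeginPlay.
; FindEnemyToLook line-traces from the head for visibility, but resets its distance threshold every iteration, so the last qualifying enemy wins over the nearest.
; LookAtEnemy smoothly rotates the head toward that target; nothing here calls it.
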(event OnComponentBeginOverlap(AttackRadius)
  (params (OverlappedComponent :type Primitive%20Component%20Object%20Reference) (OtherActor :type Actor%20Object%20Reference) (OtherComp :type Primitive%20Component%20Object%20Reference) (OtherBodyIndex :type Integer) (bFromSweep :type Boolean) (SweepResult :type Hit%20Result%20Structure%20%28by%20ref%29))
  (if (Actor|ActorHasTag OtherActor (Variables|Default|GetEnemyTag))
    (Utilities|Array|AddUnique (Variables|Default|GetEnemy) OtherActor)))

(event OnComponentEndOverlap(AttackRadius)
  (params (OverlappedComponent :type Primitive%20Component%20Object%20Reference) (OtherActor :type Actor%20Object%20Reference) (OtherComp :type Primitive%20Component%20Object%20Reference) (OtherBodyIndex :type Integer))
  (if (Actor|ActorHasTag OtherActor (Variables|Default|GetEnemyTag))
    (Utilities|Array|RemoveItem (Variables|Default|GetEnemy) OtherActor)
    (if true
      _)))

(event Custom|FindEnemyToLook
  (bind _head (Variables|Default|GetHead))
  (bind _returnvalue (Transformation|GetWorldLocation _head))
  (if (Utilities|Array|IsEmpty (Variables|Default|GetEnemy))
    (Variables|Default|SetNearestEnemy 0)
    (Variables|Default|SetNearestLength 9999.0)
    (else
      (for _array_element (Variables|Default|GetEnemy)
        (bind (_outhit _returnvalue_2) (Collision|LineTraceByChannel _returnvalue (Transformation|GetActorLocation _array_element) "TraceTypeQuery1" false (Utilities|Array|MakeArray _array_element) "None"))
        (Variables|Default|SetNearestLength (* (Variables|Default|GetAttack%20Radius) 3.0))
        (if (not _returnvalue_2)
          (if (> (Variables|Default|GetNearestLength) (Math|Vector|VectorLength (- _returnvalue (Transformation|GetActorLocation _array_element))))
            (Variables|Default|SetNearestLength (Math|Vector|VectorLength (- _returnvalue (Transformation|GetActorLocation _array_element))))
            (Variables|Default|SetNearestEnemy _array_element)))))))

(event EventBeginPlay
  (Components|Sphere|SetSphereRadius (Variables|Default|GetAttackRadius) (Variables|Default|GetAttack%20Radius) true)
  (bind _returnvalue (Utilities|Time|SetTimerbyEvent (EventDispatchers|CreateEvent :!event Custom|FindEnemyToLook) 0.1 true))
  (Variables|Default|SetLookAtEnemyHandle _returnvalue))

(event Collision|EventActorBeginOverlap
  (params (OtherActor :type Actor%20Object%20Reference)))

(fn ConstructionScript)

(fn LookatEnemy
  (params (DeltaTime :type Float%20%28single-precision%29))
  (Transformation|SetRelativeRotation (Variables|Default|GetHead) (Math|Interpolation|RInterpTo (Variables|/Script/Engine.SceneComponent|GetRelativeRotation (Variables|Default|GetHead)) (Math|Rotator|FindLookatRotation (Transformation|GetWorldLocation (Variables|Default|GetHead)) (Transformation|GetActorLocation (Variables|Default|GetNearestEnemy))) DeltaTime 4e+01) false false)
  (return))