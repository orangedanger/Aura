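; Flame pillar actor that makes its point light flicker like fire.
; On BeginPlay it sets the light to a base intensity and picks one of two flame timelines at random.
; Each timeline's intensity curve scales that base value every update, and on finishing triggers another random pick, producing an endless, varied flicker without Tick.
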(event Custom|Flame%20Effect_2
  (bind _intensity (Timeline|FlameEffect_2 PlayFromStart)
    (:Update
      (Rendering|Components|Light|SetIntensity (Variables|Default|GetPointLight) (* _intensity (Variables|Default|GetBaseInternsity))))
    (:Finished
      (CallFunction|SelectRandomFlame))))

(event Custom|Flame%20Effect_1
  (bind _intensity (Timeline|FlameEffect_1 PlayFromStart)
    (:Update
      (Rendering|Components|Light|SetIntensity (Variables|Default|GetPointLight) (* _intensity (Variables|Default|GetBaseInternsity))))
    (:Finished
      (CallFunction|SelectRandomFlame))))

(event Custom|SelectRandomFlame
  (switch int (Math|Random|RandomIntegerinRange 0 1)
    (:0
      (CallFunction|FlameEffect1))
    (:1
      (CallFunction|FlameEffect2))))

(event EventBeginPlay
  (Rendering|Components|Light|SetIntensity (Variables|Default|GetPointLight) (Variables|Default|GetBaseInternsity))
  (CallFunction|SelectRandomFlame))

(fn ConstructionScript)