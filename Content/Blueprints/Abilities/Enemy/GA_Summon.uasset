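; Enemy gameplay ability that summons minions: the avatar faces its combat target and plays the montage tagged Montage.Summon.Weapon.
; The montage's gameplay event triggers ground Niagara effects at random summon locations, then a delayed loop spawns random-class characters there with default controllers.
; Each spawn increments the summoner's minion count, and its OnDestroyed callback decrements it.
; EndAbility is wired only to montage interruption or cancellation.
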(event Custom|OnDestroyed_事件
  (params (DestroyedActor :type Actor%20Object%20Reference))
  (Class|CombatInterface|SetMinionCount(Message) (Ability|GetAvatarActorfromActorInfo) -1))

(event Ability|EventActivateAbility
  (bind _returnvalue (Ability|GetAvatarActorfromActorInfo))
  (bind _returnvalue_2 (Class|EnemyInterface|GetCombatTarget(Message) _returnvalue))
  (bind _ascombat_interface (Utilities|Casting|CastToCombatInterface _returnvalue))
  (Class|CombatInterface|SetFacingTarget _ascombat_interface (Transformation|GetActorLocation _returnvalue_2))
  (bind _returnvalue_3 (Class|AuraAbilitySystemLibrary|GetMontagefromArraybyTag (Class|CombatInterface|GetAttackMontages _ascombat_interface) "(TagName=\"Montage.Summon.Weapon\")"))
  (bind _output_get (Variables|Default|SetMontage _returnvalue_3))
  (|PlayMontageandWaitProxy "None" (.AttackMontage (Utilities|Struct|BreakTaggedMontage _output_get)) 1.0 "None" false 1.0 0.0 false
    (:then
      (Ability|Tasks|WaitGameplayEvent (.MontageTag (Utilities|Struct|BreakTaggedMontage _output_get)) 0 true
        (:EventReceived
          (bind _returnvalue_4 (Class|AuraSummonGameplayAbility|GetRandomSummonLocation))
          (bind _output_get_2 (Variables|Default|SetRandomLocations _returnvalue_4))
          (for _array_element _output_get_2
            (Niagara|SpawnSystematLocation "/Game/Assets/Effects/Combat/NS_GroundSummon.NS_GroundSummon" _array_element))
          (Utilities|FlowControl|Delay 0.5)
          (if (< (Variables|Default|GetSpawnLocationIndex) (Utilities|Array|Length (Variables|Default|GetRandomLocations))) :!label _label
            (bind _returnvalue_5 (Game|SpawnActorfromClass (Class|AuraSummonGameplayAbility|GetRandomCHaracterClass) (Math|Transform|MakeTransform (+ (Utilities|Array|Get(acopy) (Variables|Default|GetRandomLocations) (Variables|Default|GetSpawnLocationIndex)) "0.000000,0.000000,60.000000") (Math|Rotator|FindLookatRotation (Transformation|GetActorLocation (Ability|GetAvatarActorfromActorInfo)) (+ (Utilities|Array|Get(acopy) (Variables|Default|GetRandomLocations) (Variables|Default|GetSpawnLocationIndex)) "0.000000,0.000000,60.000000")) "1.000000,1.000000,1.000000") "AlwaysSpawn" "MultiplyWithRoot" 0 0))
            (Pawn|SpawnDefaultController _returnvalue_5)
            (Game|AssignOnDestroyed _returnvalue_5 (delegate Custom|OnDestroyed_事件))
            (Math|Integer|IncrementInt (Variables|Default|GetSpawnLocationIndex)
              (:%20%20
                (Class|CombatInterface|SetMinionCount(Message) (Ability|GetAvatarActorfromActorInfo) 1)
                (Utilities|FlowControl|Delay 0.2)
                (goto _label)))))))
    (:OnInterrupted
      (Ability|EndAbility :!label _label_2))
    (:OnCancelled
      (goto _label_2))))

(event Ability|EventOnEndAbility
  (params (bWasCancelled :type Boolean)))