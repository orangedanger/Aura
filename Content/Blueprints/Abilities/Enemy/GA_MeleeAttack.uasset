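; Enemy melee attack ability that faces the combat target and plays a random attack montage.
; The montage's tagged gameplay event triggers a small sphere query at that tag's weapon socket, ignoring all BP_Enemy actors.
; Found actors take damage if the combat target, rather than each found actor, is not a friend.
; A hit fires the MeleeImpact cue with the montage tag; the ability ends after the check or when the montage finishes.
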(event Ability|EventActivateAbility
  (bind _returnvalue (Ability|GetAvatarActorfromActorInfo))
  (bind _returnvalue_2 (Ability|GetAvatarActorfromActorInfo))
  (Variables|Default|SetbHitTarget false)
  (bind _returnvalue_3 (Class|EnemyInterface|GetCombatTarget(Message) _returnvalue_2))
  (bind _output_get (Variables|Default|SetCombat%20Target _returnvalue_3))
  (bind _ascombat_interface (Utilities|Casting|CastToCombatInterface _returnvalue_2))
  (Class|CombatInterface|SetFacingTarget _ascombat_interface (Transformation|GetActorLocation _output_get))
  (bind _returnvalue_4 (Class|AuraAbilitySystemLibrary|GetRandomMontagefromArray (Class|CombatInterface|GetAttackMontages _ascombat_interface)))
  (|PlayMontageandWaitProxy "None" (.AttackMontage (Utilities|Struct|BreakTaggedMontage _returnvalue_4)) 1.0 "None" false 1.0 0.0 false
    (:then
      (Ability|Tasks|WaitGameplayEvent (.MontageTag (Utilities|Struct|BreakTaggedMontage _returnvalue_4)) 0
        (:EventReceived
          (bind _returnvalue_5 (Class|CombatInterface|GetWeaponSocketLocation(Message) _returnvalue (.MontageTag (Utilities|Struct|BreakTaggedMontage _returnvalue_4))))
          (bind _output_get_2 (Variables|Default|SetSocket%20Location _returnvalue_5))
          (bind _outactors (Actor|GetAllActorsOfClass "/Game/Blueprints/AuraEnemy/BP_Enemy.BP_Enemy_C"))
          (bind _outputactor (Class|AuraAbilitySystemLibrary|QueryActorsinRadius _returnvalue _outactors 6e+01 _output_get_2))
          (for _array_element _outputactor
            (bind _returnvalue_6 (Class|AuraAbilitySystemLibrary|IsNotFriends _returnvalue (Variables|Default|GetCombat%20Target)))
            (if _returnvalue_6
              (Class|AuraDamageGameplayAbility|CasusDamage _array_element)
              (Variables|Default|SetbHitTarget true)))
          (if (Variables|Default|GetbHitTarget)
            (Class|GameplayAbility|ExecuteGameplayCuewithParams "(TagName=\"GameplayCue.MeleeImpact\")" (Ability|GameplayCue|MakeGameplayCueParameters :AggregatedSourceTags (GameplayTags|MakeGameplayTagContainerfromTag (.MontageTag (Utilities|Struct|BreakTaggedMontage _returnvalue_4))) :Location (Variables|Default|GetSocket%20Location) :Instigator (Variables|Default|GetCombat%20Target) :EffectCauser (Ability|GetAvatarActorfromActorInfo)))
            (Ability|EndAbility)
            (else
              (Ability|EndAbility))))))
    (:OnCompleted
      (Ability|EndAbility :!label _label))
    (:OnInterrupted
      (goto _label))
    (:OnCancelled
      (goto _label))))

(event Ability|EventOnEndAbility
  (params (bWasCancelled :type Boolean)))