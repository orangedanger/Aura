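; Gameplay ability for a ranged enemy attack that fires a projectile at the avatar's combat target.
; On activation it turns the avatar to face the target, then re-rolls random attack montages until one's tag matches Montage.Attack and plays it.
; A gameplay event carrying that montage's tag triggers ProjectileShell toward the target's location.
; The ability ends when the montage completes, is interrupted or is cancelled.
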(event Ability|EventOnEndAbility
  (params (bWasCancelled :type Boolean)))

(event Ability|EventActivateAbility
  (bind _returnvalue (Ability|GetAvatarActorfromActorInfo))
  (bind _returnvalue_2 (Class|EnemyInterface|GetCombatTarget(Message) _returnvalue))
  (bind _ascombat_interface (Utilities|Casting|CastToCombatInterface _returnvalue))
  (Class|CombatInterface|SetFacingTarget _ascombat_interface (Transformation|GetActorLocation _returnvalue_2))
  (bind _returnvalue_3 (Class|AuraAbilitySystemLibrary|GetRandomMontagefromArray (Class|CombatInterface|GetAttackMontages _ascombat_interface) :!label _label))
  (if (GameplayTags|MatchesTag (.MontageTag (Utilities|Struct|BreakTaggedMontage _returnvalue_3)) "(TagName=\"Montage.Attack\")")
    (Variables|Default|SetMontage _returnvalue_3)
    (|PlayMontageandWaitProxy "None" (.AttackMontage (Utilities|Struct|BreakTaggedMontage _returnvalue_3)) 1.0 "None" false 1.0 0.0 false
      (:then
        (Ability|Tasks|WaitGameplayEvent (.MontageTag (Utilities|Struct|BreakTaggedMontage _returnvalue_3)) 0 true
          (:EventReceived
            (Class|AuraProjectileSpell|ProjectileShell (Transformation|GetActorLocation _returnvalue_2) (.MontageTag (Utilities|Struct|BreakTaggedMontage _returnvalue_3))))))
      (:OnCompleted
        (Ability|EndAbility :!label _label_2))
      (:OnInterrupted
        (goto _label_2))
      (:OnCancelled
        (goto _label_2)))
    (else
      (goto _label))))