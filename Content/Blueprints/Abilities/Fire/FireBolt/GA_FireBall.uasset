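; Fireball gameplay ability that casts toward the point under the mouse.
; On activation it commits, gets cursor target data, turns the avatar to that hit location through CombatInterface and plays the cast montage.
; A Montage.Attack.Weapon gameplay event times the ProjectileShell call with that location and weapon tag.
; The ability ends shortly after that call, or immediately if the montage is interrupted or cancelled.
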(event Ability|EventActivateAbility
  (bind _returnvalue (GameplayTags|MakeLiteralGameplayTag "(TagName=\"Montage.Attack.Weapon\")"))
  (Ability|CommitAbility)
  (bind _datahandle (|UnderMouseTargetData)
    (:ValidData
      (Variables|Default|SetLocation (.Location (Collision|BreakHitResult (Ability|TargetData|GetHitResultfromTargetData _datahandle))))
      (bind _ascombat_interface (Utilities|Casting|CastToCombatInterface (Ability|GetAvatarActorfromActorInfo)))
      (Class|CombatInterface|SetFacingTarget _ascombat_interface (Variables|Default|GetLocation))
      (|PlayMontageandWaitProxy "None" "/Game/Assets/Characters/Aura/Animations/Abilities/AM_Cast_FireBall.AM_Cast_FireBall" 1.0 "None" true 1.0 0.0 false
        (:then
          (Ability|Tasks|WaitGameplayEvent _returnvalue 0
            (:EventReceived
              (Class|AuraProjectileSpell|ProjectileShell (Variables|Default|GetLocation) _returnvalue)
              (Utilities|FlowControl|Delay 0.5)
              (Ability|EndAbility))))
        (:OnInterrupted
          (Ability|EndAbility :!label _label))
        (:OnCancelled
          (goto _label))))))

(event Ability|EventOnEndAbility
  (params (bWasCancelled :type Boolean)))